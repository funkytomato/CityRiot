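; Zombie NPC character that spawns with randomized scale, yaw and walk speed, takes damage and dies.
; Damage lowers clamped health, then either plays a random left-hit montage with movement paused or stops AI logic and ragdolls before destroying itself.
; An attack box toggles CanAttack while the player overlaps it.
; Takedown events line-trace for a player character, snap behind it with the camera boom on the spine, and play montages.
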(event OnComponentBeginOverlap(AttackBox)
  (params (OverlappedComponent :type Primitive%20Component%20Object%20Reference) (OtherActor :type Actor%20Object%20Reference) (OtherComp :type Primitive%20Component%20Object%20Reference) (OtherBodyIndex :type Integer) (bFromSweep :type Boolean) (SweepResult :type Hit%20Result%20Structure%20%28by%20ref%29))
  ;[1 1 1] Is Player within Attack Box?
  (Utilities|Casting|CastToZombieTDCharacter OtherActor)
  (Variables|Default|SetCanAttack? true))

(event OnComponentEndOverlap(AttackBox)
  (params (OverlappedComponent :type Primitive%20Component%20Object%20Reference) (OtherActor :type Actor%20Object%20Reference) (OtherComp :type Primitive%20Component%20Object%20Reference) (OtherBodyIndex :type Integer))
  ;[1 1 1] Is Player within Attack Box?
  (Utilities|Casting|CastToZombieTDCharacter OtherActor)
  (Variables|Default|SetCanAttack? false))

(event Custom|TakedownSequence
  ;[1 1 1] Takedown Sequence
  (Pawn|Components|CharacterMovement|DisableMovement (Variables|Character|GetCharacterMovement))
  (Collision|SetActorEnableCollision false)
  (Animation|PlayAnimMontage 0 1.0 "None")
  (Utilities|FlowControl|Delay 1e+01)
  (Actor|DestroyActor))

(event Custom|OnDeath
  (bind _mesh (Variables|Character|GetMesh))
  ;[1 1 1] OnDeath - Play death sequence and animation
  (AI|Logic|StopLogic (Variables|/Script/AIModule.AIController|GetBrainComponent (AI|GetAIController self)) "")
  (Collision|SetCollisionProfileName _mesh "Ragdoll" true :!class /Script/Engine.PrimitiveComponent)
  (Physics|SetSimulatePhysics _mesh true)
  (Collision|SetCollisionProfileName (Variables|Collision|GetCapsuleComponent) "NoCollision" true :!class /Script/Engine.PrimitiveComponent)
  (Utilities|FlowControl|Delay 5.0)
  (Actor|DestroyActor))

(event Custom|OnHit
  (params (direction :type HitDirectionEnum%20Enum :default "NewEnumerator0"))
  (bind _hitfromleftmontages (Variables|Default|GetHitFromLeftMontages))
  (bind _hitfromrightmontages (Variables|Default|GetHitFromRightMontages))
  (bind _hitfromcentremontages (Variables|Default|GetHitFromCentreMontages))
  ;[1 1 1] Play Hit Montage respective of direction
  (Pawn|Components|CharacterMovement|DisableMovement (Variables|Character|GetCharacterMovement))
  (switch Utilities|FlowControl|Switch|SwitchonHitDirectionEnum direction
    (:NewEnumerator0
      (bind _returnvalue (Animation|Montage|MontagePlay (Variables|Default|GetAnimInstanceRef) (Utilities|Array|Get(acopy) _hitfromleftmontages (Math|Random|RandomIntegerinRange 0 (Utilities|Array|Length _hitfromleftmontages))) 1.0 "MontageLength" 0.0 true))
      (Utilities|FlowControl|Delay _returnvalue)
      (Pawn|Components|CharacterMovement|SetMovementMode (Variables|Character|GetCharacterMovement) "MOVE_Walking" 0))
    (:NewEnumerator1
      (bind _returnvalue_2 (Animation|Montage|MontagePlay (Variables|Default|GetAnimInstanceRef) (Utilities|Array|Get(acopy) _hitfromrightmontages (Math|Random|RandomIntegerinRange 0 (Utilities|Array|Length _hitfromrightmontages))) 1.0 "MontageLength" 0.0 true))
      (Utilities|FlowControl|Delay _returnvalue_2)
      (Pawn|Components|CharacterMovement|SetMovementMode (Variables|Character|GetCharacterMovement) "MOVE_Walking" 0))
    (:NewEnumerator2
      (bind _returnvalue_3 (Animation|Montage|MontagePlay (Variables|Default|GetAnimInstanceRef) (Utilities|Array|Get(acopy) _hitfromcentremontages (Math|Random|RandomIntegerinRange 0 (Utilities|Array|Length _hitfromcentremontages))) 1.0 "MontageLength" 0.0 true))
      (Utilities|FlowControl|Delay _returnvalue_3)
      (Pawn|Components|CharacterMovement|SetMovementMode (Variables|Character|GetCharacterMovement) "MOVE_Walking" 0))))

(event Custom|TakedownEvent
  (bind _returnvalue (Transformation|GetActorLocation))
  ;[1 1 1] Takedown Event - Check target can be taken down, take them down
  (if (Variables|Default|GetCanTakeDown?)
    (bind (_outhit _returnvalue_2) (Collision|LineTraceByChannel _returnvalue (+ _returnvalue (* (Transformation|GetActorForwardVector) 2.5e+02)) "TraceTypeQuery1" false 0 "None"))
    (if _returnvalue_2
      (bind _aszombie_tdcharacter (Utilities|Casting|CastToZombieTDCharacter (.HitActor (Collision|BreakHitResult _outhit))))
      (Variables|Default|SetTakedownTarget _aszombie_tdcharacter)
      (Transformation|AttachComponentToComponent (Variables|Default|GetCameraBoom) (Variables|Character|GetMesh) "spine_02" "SnapToTarget" "SnapToTarget" "SnapToTarget" true)
      (Pawn|Components|CharacterMovement|DisableMovement (Variables|Character|GetCharacterMovement))
      (Variables|Default|SetCanTakeDown? false)
      (Transformation|SetActorTransform (Math|Transform|MakeTransform (+ (.location (Transformation|GetActorTransform (Variables|Default|GetTakedownTarget))) (* (Transformation|GetActorForwardVector (Variables|Default|GetTakedownTarget)) -175.0)) (.rotation (Transformation|GetActorTransform (Variables|Default|GetTakedownTarget))) "1,1,1"))
      (bind _returnvalue_3 (Animation|PlayAnimMontage 0 1.0 "None"))
      (CallFunction|TakedownSequence)
      (Utilities|FlowControl|Delay (+ _returnvalue_3 0.025))
      (Transformation|SetActorLocation (+ (Transformation|GetActorLocation) (* (Transformation|GetActorForwardVector) 175.0)) false false)
      (Pawn|Components|CharacterMovement|SetMovementMode (Variables|Character|GetCharacterMovement) "MOVE_Walking" 0)
      (Transformation|AttachComponentToComponent (Variables|Default|GetCameraBoom) (Variables|Collision|GetCapsuleComponent) "None" "KeepRelative" "KeepRelative" "KeepRelative" true))))

(event EventBeginPlay
  (bind _returnvalue (Math|Random|RandomFloatinRange 0.9 1.1))
  ;[1 1 1] BeginPlay, Random scale and rotation of Zombie
  (Transformation|SetWorldScale3D (Variables|Character|GetMesh) (Math|Vector|MakeVector _returnvalue _returnvalue _returnvalue))
  (Transformation|SetActorRotation (Math|Rotator|MakeRotator 0.0 0.0 (Math|Random|RandomFloatinRange 0.0 3.6e+02)))
  (Variables|/Script/Engine.CharacterMovementComponent|SetMaxWalkSpeed (Variables|Character|GetCharacterMovement) (Math|Random|RandomFloatinRange 4.5e+02 7.5e+02))
  (bind _aszombie_anim_bp (Utilities|Casting|CastToZombie_AnimBP (Components|SkeletalMesh|GetAnimInstance (Variables|Character|GetMesh))))
  (Variables|Default|SetAnimInstanceRef _aszombie_anim_bp))

(event Game|Damage|EventAnyDamage
  (params (Damage :type Float%20%28single-precision%29) (DamageType :type Damage%20Type%20Object%20Reference) (InstigatedBy :type Controller%20Object%20Reference) (DamageCauser :type Actor%20Object%20Reference))
  ;[1 1 1] Damage
  (CallFunction|DecreaseHealth Damage)
  (Development|PrintString "Zombie damage received")
  (if (Variables|Default|GetIsDead?)
    (CallFunction|OnDeath)
    (else
      (CallFunction|OnHit "NewEnumerator0"))))

(event Collision|EventHit
  (params (MyComp :type Primitive%20Component%20Object%20Reference) (Other :type Actor%20Object%20Reference) (OtherComp :type Primitive%20Component%20Object%20Reference) (bSelfMoved :type Boolean) (HitLocation :type Vector :default "0, 0, 0") (HitNormal :type Vector :default "0, 0, 0") (NormalImpulse :type Vector :default "0, 0, 0") (Hit :type Hit%20Result%20Structure%20%28by%20ref%29))
  ;[1 1 1] Damage
  (Development|PrintString "Hello"))

(fn ConstructionScript)

(fn IncreaseHealth
  (params (amount :type Float%20%28single-precision%29))
  (Variables|Default|SetHealth (Math|Float|Clamp(Float) (- (Variables|Default|GetHealth) amount) 0.0 1e+02)))

(fn DecreaseHealth
  (params (amount :type Float%20%28single-precision%29))
  (bind _output_get (Variables|Default|SetHealth (Math|Float|Clamp(Float) (- (Variables|Default|GetHealth) amount) 0.0 1e+02)))
  (if (> _output_get 0.0)
    (Development|PrintString "dead")
    (else
      (Variables|Default|SetIsDead? true))))